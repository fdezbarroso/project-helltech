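; BP_Damageable is a health component that handles damage and death for its owning actor, either player or enemy.
; Health starts at MaxHealth, and SubstractHealth applies clamped damage, returning true when the hit is lethal.
; An Enemy flag passed with each hit picks the death path: enemies are hidden, lose collision, play a 2D sound and are destroyed.
; Player death opens the Died_menu level.
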(event `self.ReceiveBeginPlay`
  (set `self.Health` (`self.MaxHealth`)))

(event `DeathPlayer`
  (`GameplayStatics.OpenLevel` "Died_menu"))

(event `DeathEnemy`
  (bind _returnvalue (`self.GetOwner`))
  (`Actor.SetActorHiddenInGame` _returnvalue true)
  (`Actor.SetActorEnableCollision` _returnvalue false)
  (`GameplayStatics.PlaySound2D` "/Game/HellTech/Sounds/DeathEnemy1.DeathEnemy1" 1.0 1.0 0.0 null null)
  (`Actor.K2_DestroyActor` (`self.GetOwner`)))

(fn `SubstractHealth`
  (params (Damage :type "Float (double-precision)") (Enemy :type Boolean))
  (returns (IsDeath :type Boolean))
  (bind _returnvalue (`KismetMathLibrary.FClamp` (- (`self.Health`) Damage) 0.0 (`self.MaxHealth`)))
  (if (<= _returnvalue 0.0)
    (if Enemy
      (`self.DeathEnemy`)
      (else
        (`self.DeathPlayer`)))
    (return true)
    (else
      (set `self.Health` _returnvalue)
      (return false))))