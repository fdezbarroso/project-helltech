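; BP_Barrier is a toggleable barrier that starts invisible and without collision.
; ActiveBarrier and DesactiveBarrier switch the Plane's collision immediately, then play a fade timeline that drives the Opacity parameter of a dynamic material created at BeginPlay.
; An Activated flag, set during timeline updates, guards against repeated activation or deactivation.
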(event `self.ReceiveBeginPlay`
  (bind _plane (`self.Plane`))
  (`PrimitiveComponent.SetCollisionEnabled` (`self.Plane`) "NoCollision")
  (bind _returnvalue (`PrimitiveComponent.CreateDynamicMaterialInstance` _plane 0 (`PrimitiveComponent.GetMaterial` _plane 0) "None"))
  (bind _output_get (set `self.DynamicMaterial` _returnvalue))
  (`MaterialInstanceDynamic.SetScalarParameterValue` _output_get "Opacity" 0.0))

(event `ActiveBarrier`
  (if (not (`self.Activated?`))
    (`PrimitiveComponent.SetCollisionEnabled` (`self.Plane`) "QueryAndPhysics")
    (bind (_direction _opacity) (`Timeline|FadeIn` :!via `PlayFromStart`)
      (:`Update`
        (`MaterialInstanceDynamic.SetScalarParameterValue` (`self.DynamicMaterial`) "Opacity" _opacity)
        (set `self.Activated?` true)))))

(event `DesactiveBarrier`
  (if (`self.Activated?`)
    (`PrimitiveComponent.SetCollisionEnabled` (`self.Plane`) "NoCollision")
    (bind (_direction _opacidad) (`Timeline|FadeOut` :!via `PlayFromStart`)
      (:`Update`
        (`MaterialInstanceDynamic.SetScalarParameterValue` (`self.DynamicMaterial`) "Opacity" _opacidad)
        (set `self.Activated?` false)))))

(fn `UserConstructionScript`)