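; BP_ActivationZone is a one-shot trigger volume that fires an activation when something overlaps its Box component.
; The overlap calls Active and then destroys the actor, with no check on what entered.
; Active only forwards to the parent implementation, so the actual activation behavior lives outside this Blueprint.
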(event `self.Active`
  (`parent.Active`))

(event `self.Box.OnComponentBeginOverlap`
  (params (OverlappedComponent :type "PrimitiveComponent Object Reference") (OtherActor :type "Actor Object Reference") (OtherComp :type "PrimitiveComponent Object Reference") (OtherBodyIndex :type Integer) (bFromSweep :type Boolean) (SweepResult :type "HitResult Structure (by ref)"))
  (`self.Active`)
  (`self.K2_DestroyActor`))

(fn `UserConstructionScript`
  (`parent.UserConstructionScript`))