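; BP_ActivableWall is an activable wall actor that disappears when activated, opening the way it occupied.
; Its Active event calls the parent implementation, then hides the actor in game and disables its collision.
; The wall is never destroyed, and BeginPlay, overlap and Tick are disabled stubs.
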(event `self.Active`
  (`parent.Active`)
  (`self.SetActorHiddenInGame` true)
  (`self.SetActorEnableCollision` false))

(fn `UserConstructionScript`
  (`parent.UserConstructionScript`))