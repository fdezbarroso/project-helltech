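; BP_Enemy is a suicide-bomber enemy that chases the first-person player and explodes.
; Pawn sensing of sight or noise drives AIMoveTo, whose success flags the mesh through custom primitive data and enables the Explosion collision.
; A player overlap then starts a fuse delay, after which it spawns BP_Exploud, damages that player without rechecking range, and destroys itself.
; Incoming damage is forwarded to BPDamageable to subtract health.
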(event `self.ReceiveBeginPlay`
  (bind _mesh (`self.Mesh`))
  (`PrimitiveComponent.SetCollisionEnabled` (`self.Explosion`) "NoCollision")
  (bind _returnvalue (`PrimitiveComponent.CreateDynamicMaterialInstance` _mesh 0 (`PrimitiveComponent.GetMaterial` _mesh 0) "None"))
  (set `self.DynamicMaterial` _returnvalue)
  (`PrimitiveComponent.SetDefaultCustomPrimitiveDataFloat` (`self.Mesh`) 0 0.0))

(event `self.PawnSensing.OnSeePawn`
  (params (Pawn :type "Pawn Object Reference"))
  (bind _asbp_first_person_prototype (cast `/Game/HellTech/Blueprints/BP_FirstPersonPrototype` Pawn))
  (`|AIMoveTo` self (0.0 0.0 0.0) _asbp_first_person_prototype 200.0
    (:`OnSuccess`
      (`self.Exploud` :!label _label))))

(event `self.PawnSensing.OnHearNoise`
  (params (Instigator :type "Pawn Object Reference") (Location :type "Vector Structure (by ref)") (Volume :type "Float (single-precision)"))
  (bind _asbp_first_person_prototype (cast `/Game/HellTech/Blueprints/BP_FirstPersonPrototype` Instigator))
  (`|AIMoveTo` self (0.0 0.0 0.0) _asbp_first_person_prototype 200.0
    (:`OnSuccess`
      (goto _label))))

(event `self.ReceiveAnyDamage`
  (params (Damage :type "Float (single-precision)") (DamageType :type "DamageType Object Reference") (InstigatedBy :type "Controller Object Reference") (DamageCauser :type "Actor Object Reference"))
  (`/Game/HellTech/Blueprints/BP_Damageable.SubstractHealth` (`self.BP_Damageable`) Damage))

(event `Exploud`
  (`PrimitiveComponent.SetCustomPrimitiveDataFloat` (`self.Mesh`) 0 1.0)
  (`PrimitiveComponent.SetCollisionEnabled` (`self.Explosion`) "QueryOnly"))

(event `self.Explosion.OnComponentBeginOverlap`
  (params (OverlappedComponent :type "PrimitiveComponent Object Reference") (OtherActor :type "Actor Object Reference") (OtherComp :type "PrimitiveComponent Object Reference") (OtherBodyIndex :type Integer) (bFromSweep :type Boolean) (SweepResult :type "HitResult Structure (by ref)"))
  (bind _asbp_first_person_prototype (cast `/Game/HellTech/Blueprints/BP_FirstPersonPrototype` OtherActor))
  (`KismetSystemLibrary.Delay` (`self.TimeToExploud`))
  (`|SpawnActorFromClass` "/Game/HellTech/Blueprints/BP_Exploud.BP_Exploud_C" (`KismetMathLibrary.Conv_VectorToTransform` (`self.K2_GetActorLocation`)) "AlwaysSpawn" "MultiplyWithRoot" null null)
  (`GameplayStatics.ApplyDamage` _asbp_first_person_prototype (`self.ExplosionDamage`))
  (`KismetSystemLibrary.Delay` 1.0)
  (`self.K2_DestroyActor`))

(fn `UserConstructionScript`)